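; BP_BaseZombie is a zombie that attacks survivors and is destroyed when its health runs out.
; Damage it takes is forwarded to its Health component, whose OnDeath event destroys the actor.
; Each tick it reads the Survivor from its Blackboard and, when that BP_Survivor is within attack radius and the attack interval has elapsed, applies damage and resets the timer.
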(event `self.ReceiveBeginPlay`
  (add `self.OnTakeAnyDamage` (delegate `OnTakeAnyDamage_Event`)))

(event `OnTakeAnyDamage_Event` :!signature `self.OnTakeAnyDamage`
  (params (DamagedActor :type "Actor Object Reference") (Damage :type "Float (single-precision)") (DamageType :type "DamageType Object Reference") (InstigatedBy :type "Controller Object Reference") (DamageCauser :type "Actor Object Reference"))
  (`HealthComponent.TakeDamage` (`self.Health`) (`KismetMathLibrary.FTrunc` Damage)))

(event `self.Health.OnDeath`
  (`self.K2_DestroyActor`))

(event `self.ReceiveTick`
  (params (DeltaSeconds :type "Float (single-precision)"))
  (bind _returnvalue (`BlackboardComponent.GetValueAsObject` (`AIBlueprintHelperLibrary.GetBlackboard` null) "Survivor"))
  (set `self.TimeSinceLastAttack` (+ (`self.TimeSinceLastAttack`) DeltaSeconds))
  (`/Engine/EditorBlueprintResources/StandardMacros.IsValid` _returnvalue
    (:`Is Valid`
      (bind _asbp_survivor (cast `/Game/Suvivor/BP_Survivor` _returnvalue))
      (if (and (<= (`self.GetDistanceTo` _asbp_survivor self) (`self.AttackRadius`)) (> (`self.TimeSinceLastAttack`) (`self.AttackInterval`)))
        (`GameplayStatics.ApplyDamage` _asbp_survivor (`self.AttackDamage`) null self)
        (set `self.TimeSinceLastAttack` 0.0)))))

(fn `UserConstructionScript`)
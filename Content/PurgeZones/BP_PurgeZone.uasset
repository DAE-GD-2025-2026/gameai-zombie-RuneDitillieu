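; Timed purge zone that kills pawns inside a circular area, then destroys itself.
; The construction script scales the Plane to Diameter, and a dynamic material's OuterRadius shows the ratio of TimePassed to TimeTillPurge each tick.
; Once TimePassed reaches TimeTillPurge, OnPurge applies massive damage to every Pawn within half the Diameter, measured horizontally so height is ignored.
; TimePassed is read here but not advanced by these graphs.
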(event `self.ReceiveBeginPlay`
  (bind _plane (`self.Plane`))
  (bind _returnvalue (`PrimitiveComponent.CreateDynamicMaterialInstance` _plane 0 (`PrimitiveComponent.GetMaterial` _plane 0) "None"))
  (set `self.DynamicMaterial` _returnvalue))

(event `self.ReceiveTick`
  (params (DeltaSeconds :type "Float (single-precision)"))
  (`MaterialInstanceDynamic.SetScalarParameterValue` (`self.DynamicMaterial`) "OuterRadius" (`KismetMathLibrary.FClamp` (/ (`self.TimePassed`) (`self.TimeTillPurge`))))
  (if (>= (`self.TimePassed`) (`self.TimeTillPurge`))
    (`self.OnPurge`)))

(event `OnPurge`
  (bind _outactors (`GameplayStatics.GetAllActorsOfClass` "/Script/Engine.Pawn"))
  (for _array_element _outactors
    (if (<= (`self.GetHorizontalDistanceTo` _array_element self) (/ (`self.Diameter`) 2.0))
      (`GameplayStatics.ApplyDamage` _array_element 99999.0 null self)))
  (`self.K2_DestroyActor`))

(fn `UserConstructionScript`
  (`SceneComponent.SetWorldScale3D` (`self.Plane`) (`KismetMathLibrary.Conv_DoubleToVector` (/ (`self.Diameter`) 100.0))))